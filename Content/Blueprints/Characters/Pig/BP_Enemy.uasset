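; Enemy character base logic that turns around at walls and ledges.
; A WallDectect overlap prints the other actor's name and calls RotationEnemy, which flips the actor 180 degrees.
; Each Tick, after the parent's, CheckLedge calls the same flip when the movement floor is walkable but LedgeDetect overlaps no actors, treating that as a drop-off.
; Forward movement is not handled in these graphs.
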(event OnComponentBeginOverlap(WallDectect)
  (params (OverlappedComponent :type Primitive%20Component%20Object%20Reference) (OtherActor :type Actor%20Object%20Reference) (OtherComp :type Primitive%20Component%20Object%20Reference) (OtherBodyIndex :type Integer) (bFromSweep :type Boolean) (SweepResult :type Hit%20Result%20Structure%20%28by%20ref%29))
  (Development|PrintString (Utilities|GetDisplayName OtherActor))
  (CallFunction|RotationEnemy))

(event EventBeginPlay)

(event Collision|EventActorBeginOverlap
  (params (OtherActor :type Actor%20Object%20Reference)))

(event EventTick
  (params (DeltaSeconds :type Float%20%28single-precision%29))
  (|CallParentFunction DeltaSeconds)
  (CallFunction|CheckLedge))

(fn ConstructionScript
  (|CallParentFunction))

(fn RotationEnemy
  (Transformation|SetActorRotation (Math|Rotator|CombineRotators (Transformation|GetActorRotation) "0.000000,180.000000,0.000000")))

(fn CheckLedge
  (if (.bwalkablefloor (Variables|/Script/Engine.CharacterMovementComponent|GetCurrentFloor (Variables|Character|GetCharacterMovement)))
    (if (not (> (Utilities|Array|Length (Collision|GetOverlappingActors (Variables|Default|GetLedgeDetect) 0 :!class /Script/Engine.PrimitiveComponent)) 0))
      (CallFunction|RotationEnemy))))